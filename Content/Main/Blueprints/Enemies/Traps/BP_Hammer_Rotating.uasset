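; BP_Hammer_Rotating is a spinning hammer trap that knocks the player away and damages them on contact.
; BeginPlay applies its RotationRate to the RotatingMovement component on a single axis.
; A mesh hit on the player launches them away from the mesh with a slight upward bias, scaled by LaunchMultiplier, then applies Damage.
; A DoOnce, reset by a short timer, prevents repeated hits from one contact.
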(event OnComponentHit(SM_obstacle_2_001)
  (params (HitComponent :type Primitive%20Component%20Object%20Reference) (OtherActor :type Actor%20Object%20Reference) (OtherComp :type Primitive%20Component%20Object%20Reference) (NormalImpulse :type Vector :default "0, 0, 0") (Hit :type Hit%20Result%20Structure%20%28by%20ref%29))
  ;[0.15 0.15 0.15 0.5] Check if its actually hit the player
  (if (== OtherActor (Game|GetPlayerCharacter 0))
    (Utilities|FlowControl|DoOnce false
      (:Completed
        (bind _asplayer_v3 (Utilities|Casting|CastToPlayerV3 OtherActor))
        ;[0.15 0.15 0.15 0.5] Launching the player backwards on hit
        (Character|LaunchCharacter _asplayer_v3 (* (+ (- (Transformation|GetWorldLocation (Variables|/Script/Engine.Actor|GetRootComponent _asplayer_v3)) (Transformation|GetWorldLocation (Variables|Default|GetSM_obstacle_2_001))) "0.000000,0.000000,2.000000") (Variables|Default|GetLaunch%20Multiplier)) true true)
        (Game|Damage|ApplyDamage OtherActor (Variables|Stats|GetDamage) 0 0)
        (Utilities|Time|SetTimerbyFunctionName 0 "Reset" 0.2)))))

(event Custom|Reset
  (Utilities|FlowControl|DoOnce false) ; enters at Reset
)

(event EventBeginPlay
  (Variables|/Script/Engine.RotatingMovementComponent|SetRotationRate (Variables|Default|GetRotatingMovement) (Math|Rotator|MakeRotator 0.0 0.0 (Variables|Stats|GetRotation%20Rate))))

(fn ConstructionScript)