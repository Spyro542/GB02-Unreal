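; Player character that handles Enhanced Input movement, look, jumping with toggleable double jump, sprinting and melee.
; Sprint changes walk speed and camera FOV through a timeline; DoOnce-plus-delay gates pace grounded footsteps and post-hit immunity.
; Melee spawns an attached attack actor, while damage updates health stored in Playing_Instance and death respawns at the last spawnpoint.
; Interact is an empty stub, and the projectile code is unused.
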(event Input|EnhancedActionEvents|EnhancedInputActionMove
  (params (ActionValue :type Vector%202D%20Structure) (ElapsedSeconds :type Float%20%28double-precision%29) (TriggeredSeconds :type Float%20%28double-precision%29) (InputAction :type Input%20Action%20Object%20Reference :default "/Game/Main/Game_Handling/Inputs/Move.Move"))
  ;[0.15 0.15 0.15 0.5] Movement And Camera Controls
  (CallFunction|Movement (.x ActionValue) (.y ActionValue))
  (if (not (AI|Components|NavMovement|IsFalling (Variables|Character|GetCharacterMovement)))
    (Utilities|FlowControl|DoOnce false :!label _label
      (:Completed
        ;[0.15 0.15 0.15 0.5] Play Footstep Sounds  -  Running Vs Waking
        (Audio|SpawnSound2D "/Game/Main/Sound_effects/Player/Step.Step" 1.0 1.0 0.0 0)
        (if (stale Input|EnhancedActionEvents|EnhancedInputActionSprint _is_running_)
          (Utilities|FlowControl|Delay 0.25)
          (goto _label Reset)
          (else
            (Utilities|FlowControl|Delay 0.35)
            (goto _label Reset)))))))

(event Input|EnhancedActionEvents|EnhancedInputActionCamera
  (params (ActionValue :type Vector%202D%20Structure) (ElapsedSeconds :type Float%20%28double-precision%29) (TriggeredSeconds :type Float%20%28double-precision%29) (InputAction :type Input%20Action%20Object%20Reference :default "/Game/Main/Game_Handling/Inputs/Camera.Camera"))
  ;[0.15 0.15 0.15 0.5] Movement And Camera Controls
  (CallFunction|CameraControl (.x ActionValue) (.y ActionValue)))

(event Input|EnhancedActionEvents|EnhancedInputActionJump
  (params (ActionValue :type Boolean) (ElapsedSeconds :type Float%20%28double-precision%29) (TriggeredSeconds :type Float%20%28double-precision%29) (InputAction :type Input%20Action%20Object%20Reference :default "/Game/Main/Game_Handling/Inputs/Jump.Jump"))
  ;[0.15 0.15 0.15 0.5] Movement And Camera Controls
  (:Triggered
    (CallFunction|Jump ActionValue))
  (:Completed
    (Character|StopJumping)))

(event Input|EnhancedActionEvents|EnhancedInputActionSprint
  (params (ActionValue :type Boolean) (ElapsedSeconds :type Float%20%28double-precision%29) (TriggeredSeconds :type Float%20%28double-precision%29) (InputAction :type Input%20Action%20Object%20Reference :default "/Game/Main/Game_Handling/Inputs/Sprint.Sprint"))
  (bind _camera (Variables|Default|GetCamera))
  ;[0.15 0.15 0.15 0.5] Run
  (bind _is_running_ (CallFunction|Sprint ActionValue))
  ;[0.15 0.15 0.15 0.5] How Fast To Change Fov
  (bind (_direction _curve_up _curve_down) (Timeline|Timeline PlayFromStart)
    (:Update
      (if _is_running_
        ;[0.15 0.15 0.15 0.5] Set Field Of View For Sprinting And Walking
        (Camera|SetFieldOfView _camera _curve_up)
        (else
          (Camera|SetFieldOfView _camera _curve_down))))))

(event Input|EnhancedActionEvents|EnhancedInputActionInteract
  (params (ActionValue :type Boolean) (ElapsedSeconds :type Float%20%28double-precision%29) (TriggeredSeconds :type Float%20%28double-precision%29) (InputAction :type Input%20Action%20Object%20Reference :default "/Game/Main/Game_Handling/Inputs/Interact.Interact"))
  ;[0.15 0.15 0.15 0.5] To Do
  (CallFunction|Interact))

(event Input|EnhancedActionEvents|EnhancedInputActionAttack
  (params (ActionValue :type Boolean) (ElapsedSeconds :type Float%20%28double-precision%29) (TriggeredSeconds :type Float%20%28double-precision%29) (InputAction :type Input%20Action%20Object%20Reference :default "/Game/Main/Game_Handling/Inputs/Attack.Attack"))
  ;[0.15 0.15 0.15 0.5] Attack
  (CallFunction|MeeleAttack))

(event EventBeginPlay)

(event Collision|EventActorBeginOverlap
  (params (OtherActor :type Actor%20Object%20Reference)))

(event Game|Damage|EventAnyDamage
  (params (Damage :type Float%20%28single-precision%29) (DamageType :type Damage%20Type%20Object%20Reference) (InstigatedBy :type Controller%20Object%20Reference) (DamageCauser :type Actor%20Object%20Reference))
  (Utilities|FlowControl|DoOnce false :!label _label
    (:Completed
      (CallFunction|TakeDamage Damage)
      (if (>= Damage 0.0)
        (Audio|PlaySound2D "/Game/Main/Sound_effects/hitHurt.hitHurt" 1.0 1.0 0.0 0 0)
        ;[0.15 0.15 0.15 0.5] Immunity Frames
        (Utilities|FlowControl|Delay 0.2)
        (goto _label Reset)
        (else
          (goto _label Reset))))))

(event EventPossessed
  (params (NewController :type Controller%20Object%20Reference))
  ;[0.15 0.15 0.15 0.5] Set Control Mapping
  (bind _asplayer_controller (Utilities|Casting|CastToPlayerController NewController))
  (Input|AddMappingContext (PlayerController|LocalPlayerSubsystems|GetEnhancedInputLocalPlayerSubsystem _asplayer_controller) "/Game/Main/Game_Handling/Inputs/Main_Controls.Main_Controls" 0 "(bIgnoreAllPressedKeysUntilRelease=True,bForceImmediately=False,bNotifyUserSettings=False)"))

(fn ConstructionScript)

(fn Sprint
  (params (Is%20Running :type Boolean))
  (bind _charactermovement (Variables|Character|GetCharacterMovement))
  ;[0.15 0.15 0.15 0.5] Set Run And Walk Speed
  (if Is%20Running
    (Variables|/Script/Engine.CharacterMovementComponent|SetMaxWalkSpeed _charactermovement (Variables|Default|GetRun%20Speed))
    (else
      (Variables|/Script/Engine.CharacterMovementComponent|SetMaxWalkSpeed _charactermovement (Variables|Default|GetWalk%20Speed))))
  (return Is%20Running))

(fn Movement
  (params (X :type Float%20%28double-precision%29) (Y :type Float%20%28double-precision%29))
  (bind _returnvalue (Pawn|GetControlRotation :!class /Script/Engine.Pawn))
  (Pawn|Input|AddMovementInput (Math|Vector|GetRightVector (Math|Rotator|MakeRotator (.roll _returnvalue) 0.0 (.yaw _returnvalue))) X false)
  (Pawn|Input|AddMovementInput (Math|Vector|GetForwardVector (Math|Rotator|MakeRotator 0.0 0.0 (.yaw _returnvalue))) Y false))

(fn CameraControl
  (params (X :type Float%20%28double-precision%29) (Y :type Float%20%28double-precision%29))
  (Pawn|Input|AddControllerYawInput X)
  (Pawn|Input|AddControllerPitchInput Y))

(fn Jump
  (params (Button%20State :type Boolean))
  (if Button%20State
    (if (Character|CanJump)
      (Character|Jump)
      (Audio|SpawnSound2D "/Game/Main/Sound_effects/Player/Jump_Meta.Jump_Meta" 1.0 1.0 0.0 0))))

(fn MeeleAttack
  (bind _camera (Variables|Default|GetCamera))
  (bind _returnvalue (Transformation|GetWorldRotation _camera))
  (bind _returnvalue_2 (Game|SpawnActorfromClass "/Game/Main/Blueprints/Player/Meele_Test.Meele_Test_C" (Math|Transform|MakeTransform (Transformation|GetActorLocation) (Math|Rotator|MakeRotator (.roll _returnvalue) 0.0 (.yaw _returnvalue)) "1.000000,1.000000,1.000000") "Undefined" "MultiplyWithRoot" 0 0))
  (Transformation|AttachActorToActor _returnvalue_2 self "None" "KeepWorld" "KeepWorld" "KeepWorld" true)
  (Audio|SpawnSound2D "/Game/Main/Sound_effects/Player/Fire.Fire" 1.0 1.0 0.0 0))

(fn TakeDamage
  (params (Damage :type Float%20%28double-precision%29))
  (bind _asplaying_instance (Utilities|Casting|CastToPlaying_Instance (Game|GetGameInstance)))
  (bind (_current_health _max_health) (Default|UpdatePlayerCurrentHealth _asplaying_instance (Math|Float|Truncate Damage) false))
  (if (<= _current_health 0)
    (Default|UpdatePlayerCurrentHealth _asplaying_instance 0 true)
    (CallFunction|Died)
    (else
      (if (>= _current_health _max_health)
        (Default|UpdatePlayerCurrentHealth _asplaying_instance 0 true))
      (return false))))

(fn Spawnpoint
  (params (Spawnpoint :type Object%20Object%20Reference))
  (Variables|Default|SetLast%20Spawnpoint%20Visited Spawnpoint))

(fn Died
  (bind _asspawnpoint (Utilities|Casting|CastToSpawnpoint (Variables|Default|GetLast%20Spawnpoint%20Visited)))
  (Default|PlayerRespawn _asspawnpoint self))

(fn Interact)

(fn SetDoubleJump
  (params (Enable%20Double%20Jump :type Boolean))
  (if Enable%20Double%20Jump
    (Variables|Default|SetJumpMaxCount 2)
    (else
      (Variables|Default|SetJumpMaxCount 1))))