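; Fenceline is a placeable Blueprint that tiles a mesh along a spline, as for a fence line, with no runtime logic.
; The construction script measures the mesh's X bounds and divides the spline length by it to set the segment count.
; Each segment becomes a collision-enabled spline mesh component bent between consecutive distances along the spline.
; Tangents are clamped to one mesh length so each piece follows the curve.
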(event EventBeginPlay)

(event Collision|EventActorBeginOverlap
  (params (OtherActor :type Actor%20Object%20Reference)))

(event EventTick
  (params (DeltaSeconds :type Float%20%28single-precision%29)))

(fn ConstructionScript
  (bind _spline_mesh (Variables|Default|GetSpline%20Mesh))
  (bind _spline (Variables|Default|GetSpline))
  (bind _spline_2 (Variables|Default|GetSpline))
  (bind _returnvalue (StaticMesh|GetBoundingBox _spline_mesh))
  (bind (_min _max) (Utilities|Struct|BreakBox _returnvalue))
  ;[0.15 0.15 0.15 0.5] Getting The Length Of The Mesh
  (Variables|Default|SetMesh%20Length (.X (Math|Vector|BreakVector (- _max _min))))
  (for _index (range 0 (Math|Float|Truncate (/ (Spline|GetSplineLength (Variables|Default|GetSpline)) (Variables|Default|GetMesh%20Length))))
    ;[0.15 0.15 0.15 0.5] Spawn Mesh In Direction
    (bind _returnvalue_2 (AddComponent|AddSplineMeshComponent false))
    (Components|StaticMesh|SetStaticMesh _returnvalue_2 (Variables|Default|GetSpline%20Mesh))
    (SplineMesh|SetForwardAxis _returnvalue_2 "X" true)
    (SplineMesh|SetStartandEnd _returnvalue_2 (Spline|GetLocationatDistanceAlongSpline _spline (* _index (Variables|Default|GetMesh%20Length)) "Local") (Math|Vector|ClampVectorSize (Spline|GetTangentatDistanceAlongSpline _spline (* _index (Variables|Default|GetMesh%20Length)) "Local") 0.0 (Variables|Default|GetMesh%20Length)) (Spline|GetLocationatDistanceAlongSpline _spline_2 (* (+ _index 1) (Variables|Default|GetMesh%20Length)) "Local") (Math|Vector|ClampVectorSize (Spline|GetTangentatDistanceAlongSpline _spline_2 (* (+ _index 1) (Variables|Default|GetMesh%20Length)) "Local") 0.0 (Variables|Default|GetMesh%20Length)) true :!class /Script/Engine.SplineMeshComponent)
    (Collision|SetCollisionEnabled _returnvalue_2 "QueryAndPhysics")))