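; Collapsing platform Blueprint that tips over after the player character hits its obstacle mesh.
; The hit passes a DoOnce, waits a configurable delay, then plays the Rotation timeline to drive the root's world roll, keeping pitch and yaw.
; Mesh collision is off while the roll is at or below a steep threshold and on otherwise, and the timeline's end re-arms the DoOnce.
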(event OnComponentHit(SM_obstacle_5_002)
  (params (HitComponent :type Primitive%20Component%20Object%20Reference) (OtherActor :type Actor%20Object%20Reference) (OtherComp :type Primitive%20Component%20Object%20Reference) (NormalImpulse :type Vector :default "0, 0, 0") (Hit :type Hit%20Result%20Structure%20%28by%20ref%29))
  (bind _sm_obstacle_5_002 (Variables|Default|GetSM_obstacle_5_002))
  (bind _defaultsceneroot (Variables|Default|GetDefaultSceneRoot))
  (bind _returnvalue (Transformation|GetWorldRotation _defaultsceneroot))
  ;[0.15 0.15 0.15 0.5] Check if player has landed on it
  (if (== OtherActor (Game|GetPlayerCharacter 0))
    (Utilities|FlowControl|DoOnce false :!label _label
      (:Completed
        (Utilities|FlowControl|Delay (Variables|Stats|GetDelay%20before%20falling))
        (bind _rotate_down (Timeline|Rotation PlayFromStart)
          (:Update
            (Transformation|SetWorldRotation _defaultsceneroot (Math|Rotator|MakeRotator _rotate_down (.pitch _returnvalue) (.yaw _returnvalue)) false false)
            (if (<= _rotate_down -65.0)
              (Collision|SetCollisionEnabled _sm_obstacle_5_002 "NoCollision")
              (else
                (Collision|SetCollisionEnabled _sm_obstacle_5_002 "QueryAndPhysics"))))
          (:Finished
            (goto _label Reset)))))))

(event EventBeginPlay)

(event Collision|EventActorBeginOverlap
  (params (OtherActor :type Actor%20Object%20Reference)))

(event EventTick
  (params (DeltaSeconds :type Float%20%28single-precision%29)))

(fn ConstructionScript)