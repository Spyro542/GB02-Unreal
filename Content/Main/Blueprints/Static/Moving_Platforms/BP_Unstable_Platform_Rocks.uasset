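; Unstable rock platform that crumbles when the player hits it, then reassembles.
; BeginPlay saves the world location and rotation of seven rock meshes.
; A player hit passes a DoOnce, enables physics on the rocks after a delay, then disables it after another.
; Named timers then fire per-rock MoveComponentTo calls that use the saved transforms as relative targets, and a Reset timer re-arms the DoOnce.
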(event Custom|Rock%207
  (Components|MoveComponentTo (Variables|Default|GetSM_RockSmall_A7) (Variables|Location|GetRock%20location%207) (Variables|Default|GetRotation%20Rock%20_7) false false (Variables|Stats|GetReturn%20over%20time) false))

(event Custom|Rock%204
  (Components|MoveComponentTo (Variables|Default|GetSM_RockSmall_A4) (Variables|Location|GetRock%20location%204) (Variables|Default|GetRotation%20Rock%20_4) false false (Variables|Stats|GetReturn%20over%20time) false))

(event Custom|Rock%206
  (Components|MoveComponentTo (Variables|Default|GetSM_RockSmall_A6) (Variables|Location|GetRock%20location%206) (Variables|Default|GetRotation%20Rock%20_6) false false (Variables|Stats|GetReturn%20over%20time) false))

(event Custom|Reset
  (Utilities|FlowControl|DoOnce false) ; enters at Reset
)

(event Custom|Rock%205
  (Components|MoveComponentTo (Variables|Default|GetSM_RockSmall_A5) (Variables|Location|GetRock%20location%205) (Variables|Default|GetRotation%20Rock%20_5) false false (Variables|Stats|GetReturn%20over%20time) false))

(event Custom|Rock%203
  (Components|MoveComponentTo (Variables|Default|GetSM_RockSmall_A3) (Variables|Location|GetRock%20location%203) (Variables|Default|GetRotation%20Rock%20_3) false false (Variables|Stats|GetReturn%20over%20time) false))

(event Custom|Rock%202
  (Components|MoveComponentTo (Variables|Default|GetSM_RockSmall_A2) (Variables|Location|GetRock%20location%202) (Variables|Default|GetRotation%20Rock%20_2) false false (Variables|Stats|GetReturn%20over%20time) false))

(event Custom|Rock%201
  (Components|MoveComponentTo (Variables|Default|GetSM_RockSmall_A1) (Variables|Location|GetRock%20location%201) (Variables|Default|GetRotation%20Rock%20_1) false false (Variables|Stats|GetReturn%20over%20time) false))

(event EventBeginPlay
  ;[0.15 0.15 0.15 0.5] Save rock location to return to later
  (CallFunction|SaveLocationOfRocks))

(event Collision|EventHit
  (params (MyComp :type Primitive%20Component%20Object%20Reference) (Other :type Actor%20Object%20Reference) (OtherComp :type Primitive%20Component%20Object%20Reference) (bSelfMoved :type Boolean) (HitLocation :type Vector :default "0, 0, 0") (HitNormal :type Vector :default "0, 0, 0") (NormalImpulse :type Vector :default "0, 0, 0") (Hit :type Hit%20Result%20Structure%20%28by%20ref%29))
  ;[0.15 0.15 0.15 0.5] If player hit
  (if (== Other (Game|GetPlayerCharacter 0))
    (Utilities|FlowControl|DoOnce false
      (:Completed
        (Utilities|FlowControl|Delay (Variables|Stats|GetTime%20before%20crumbling))
        (CallFunction|SimulateRockPhysics true)
        (Utilities|FlowControl|Delay (Variables|Stats|GetTime%20before%20Reassembling))
        (CallFunction|SimulateRockPhysics false)
        (Utilities|Time|SetTimerbyFunctionName 0 "Rock 1" 0.1)
        (Utilities|Time|SetTimerbyFunctionName 0 "Rock 2" 0.1)
        (Utilities|Time|SetTimerbyFunctionName 0 "Rock 3" 0.1)
        (Utilities|Time|SetTimerbyFunctionName 0 "Rock 4" 0.1)
        (Utilities|Time|SetTimerbyFunctionName 0 "Rock 5" 0.1)
        (Utilities|Time|SetTimerbyFunctionName 0 "Rock 6" 0.1)
        (Utilities|Time|SetTimerbyFunctionName 0 "Rock 7" 0.1)
        (Utilities|Time|SetTimerbyFunctionName 0 "Reset" (Variables|Stats|GetReturn%20over%20time))))))

(fn ConstructionScript)

(fn SimulateRockPhysics
  (params (Enable :type Boolean))
  (Physics|SetSimulatePhysics (Variables|Default|GetSM_RockSmall_A1) Enable)
  (Physics|SetSimulatePhysics (Variables|Default|GetSM_RockSmall_A2) Enable)
  (Physics|SetSimulatePhysics (Variables|Default|GetSM_RockSmall_A3) Enable)
  (Physics|SetSimulatePhysics (Variables|Default|GetSM_RockSmall_A4) Enable)
  (Physics|SetSimulatePhysics (Variables|Default|GetSM_RockSmall_A5) Enable)
  (Physics|SetSimulatePhysics (Variables|Default|GetSM_RockSmall_A6) Enable)
  (Physics|SetSimulatePhysics (Variables|Default|GetSM_RockSmall_A7) Enable))

(fn SaveLocationOfRocks
  (bind _sm_rocksmall_a3 (Variables|Default|GetSM_RockSmall_A3))
  (bind _sm_rocksmall_a1 (Variables|Default|GetSM_RockSmall_A1))
  (bind _sm_rocksmall_a2 (Variables|Default|GetSM_RockSmall_A2))
  (bind _sm_rocksmall_a4 (Variables|Default|GetSM_RockSmall_A4))
  (bind _sm_rocksmall_a5 (Variables|Default|GetSM_RockSmall_A5))
  (bind _sm_rocksmall_a6 (Variables|Default|GetSM_RockSmall_A6))
  (bind _sm_rocksmall_a7 (Variables|Default|GetSM_RockSmall_A7))
  ;[0.15 0.15 0.15 0.5] Saving location of 7 rocks
  (Variables|Location|SetRock%20location%201 (Transformation|GetWorldLocation _sm_rocksmall_a1))
  (Variables|Location|SetRock%20location%202 (Transformation|GetWorldLocation _sm_rocksmall_a2))
  (Variables|Location|SetRock%20location%203 (Transformation|GetWorldLocation _sm_rocksmall_a3))
  (Variables|Location|SetRock%20location%204 (Transformation|GetWorldLocation _sm_rocksmall_a4))
  (Variables|Location|SetRock%20location%205 (Transformation|GetWorldLocation _sm_rocksmall_a5))
  (Variables|Location|SetRock%20location%206 (Transformation|GetWorldLocation _sm_rocksmall_a6))
  (Variables|Location|SetRock%20location%207 (Transformation|GetWorldLocation _sm_rocksmall_a7))
  ;[0.15 0.15 0.15 0.5] Saving Rock Rotations
  (Variables|Default|SetRotation%20Rock%20_1 (Transformation|GetWorldRotation _sm_rocksmall_a1))
  (Variables|Default|SetRotation%20Rock%20_2 (Transformation|GetWorldRotation _sm_rocksmall_a2))
  (Variables|Default|SetRotation%20Rock%20_3 (Transformation|GetWorldRotation _sm_rocksmall_a3))
  (Variables|Default|SetRotation%20Rock%20_4 (Transformation|GetWorldRotation _sm_rocksmall_a4))
  (Variables|Default|SetRotation%20Rock%20_5 (Transformation|GetWorldRotation _sm_rocksmall_a5))
  (Variables|Default|SetRotation%20Rock%20_6 (Transformation|GetWorldRotation _sm_rocksmall_a6))
  (Variables|Default|SetRotation%20Rock%20_7 (Transformation|GetWorldRotation _sm_rocksmall_a7)))