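; BP_Health is a health pickup that heals whatever actor overlaps its sphere by applying negative damage scaled by HealingFactor.
; A DoOnce gates the pickup, which plays a sound, hides the actor and starts a timer to restore it after ResetTime.
; Tick also polls the Playing_Instance game instance and restores the pickup while RespawnHearts is set, intended for respawning hearts on player death.
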(event OnComponentBeginOverlap(Sphere)
  (params (OverlappedComponent :type Primitive%20Component%20Object%20Reference) (OtherActor :type Actor%20Object%20Reference) (OtherComp :type Primitive%20Component%20Object%20Reference) (OtherBodyIndex :type Integer) (bFromSweep :type Boolean) (SweepResult :type Hit%20Result%20Structure%20%28by%20ref%29))
  (Utilities|FlowControl|DoOnce false
    (:Completed
      (Game|Damage|ApplyDamage OtherActor (* (Variables|Stats|GetHealing%20Factor) -1.0) 0 0)
      (Audio|PlaySound2D "/Game/Main/Sound_effects/Heal_Pickup.Heal_Pickup" 1.0 1.0 0.0 0 0)
      (Rendering|SetActorHiddenInGame true)
      (Utilities|Time|SetTimerbyFunctionName 0 "Reset" (Variables|Stats|GetReset_Time)))))

(event Custom|Reset
  (Rendering|SetActorHiddenInGame false)
  (Utilities|FlowControl|DoOnce false) ; enters at Reset
)

(event EventTick
  (params (DeltaSeconds :type Float%20%28single-precision%29))
  ;[0.15 0.15 0.15 0.5] Respawn hearts on player death
  (bind _asplaying_instance (Utilities|Casting|CastToPlaying_Instance (Game|GetGameInstance)))
  (if (Variables|/Game/Main/Game_Handling/Playing_Instance.Playing_Instance_C|GetRespawn%20Hearts _asplaying_instance)
    (Rendering|SetActorHiddenInGame false)
    (Utilities|FlowControl|DoOnce false) ; enters at Reset
  ))

(fn ConstructionScript)