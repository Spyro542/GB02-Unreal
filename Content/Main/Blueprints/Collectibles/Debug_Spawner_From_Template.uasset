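; Debug gem spawner that bursts collectible gems totaling TargetValue from its location, restarting the tally and repeating every Tick.
; A loop randomly picks 1, 5, 25 or 100-value gems, falling through to larger tiers and rerolling when the pick would overshoot the remaining value.
; Each spawned gem gets a random sideways and fixed upward force scaled by Multiplier, then resets the DoOnce gating the next pick.
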(event EventTick
  (params (DeltaSeconds :type Float%20%28single-precision%29))
  (bind _returnvalue (Math|Random|RandomFloatinRange -8e+01 8e+01))
  (bind _returnvalue_2 (Math|Random|RandomFloatinRange -8e+01 8e+01))
  (bind _returnvalue_3 (Transformation|GetActorLocation))
  (bind _multiplier (Variables|Default|GetMultiplier))
  (bind _upwards_force (Variables|Default|GetUpwards%20Force))
  (bind _returnvalue_4 (* _upwards_force _multiplier))
  (bind _returnvalue_5 (* _returnvalue_2 _multiplier))
  (bind _returnvalue_6 (* _returnvalue _multiplier))
  (Variables|Default|SetCurrent%20Value 0)
  ;[0.15 0.15 0.15 0.5] Spawn Gems Till Wanted Walue Is Achived
  (while (!= (<= (Variables|Default|GetTarget%20Value) (Variables|Default|GetCurrent%20Value)) true)
    ;[0.15 0.15 0.15 0.5] Select Gem To Spawn
    (Utilities|FlowControl|DoOnce false :!label _label
      (:Completed
        (Variables|Default|SetTemporary%20value (Math|Random|RandomIntegerinRange 1 100) :!label _label_2)
        (if (<= (Variables|Default|GetTemporary%20value) 25)
          (if (<= (Variables|Default|GetCurrent%20Value) (- (Variables|Default|GetTarget%20Value) 1))
            ;[0.15 0.15 0.15 0.5] Spawn The Selected Gem And Update Total Value Of Spawned Gems
            (bind _returnvalue_7 (Game|SpawnActorfromClass "/Game/Main/Blueprints/Collectibles/1_Gem_Collectible.1_Gem_Collectible_C" (Math|Transform|MakeTransform _returnvalue_3 "0, 0, 0" "1.000000,1.000000,1.000000") "Undefined" "MultiplyWithRoot" 0 0))
            (Physics|AddForce (Variables|/Game/Main/Blueprints/Collectibles/1_Gem_Collectible.1_Gem_Collectible_C|GetStone41 _returnvalue_7) (Math|Vector|MakeVector _returnvalue_5 _returnvalue_6 _returnvalue_4) "None" false)
            (Variables|Default|SetCurrent%20Value (+ (Variables|Default|GetCurrent%20Value) 1))
            (goto _label Reset)
            (else
              _)))
        (if (<= (Variables|Default|GetTemporary%20value) 50)
          (if (<= (Variables|Default|GetCurrent%20Value) (- (Variables|Default|GetTarget%20Value) 5))
            (bind _returnvalue_8 (Game|SpawnActorfromClass "/Game/Main/Blueprints/Collectibles/5_Gem_Collectible.5_Gem_Collectible_C" (Math|Transform|MakeTransform _returnvalue_3 "0, 0, 0" "1.000000,1.000000,1.000000") "Undefined" "MultiplyWithRoot" 0 0))
            (Physics|AddForce (Variables|/Game/Main/Blueprints/Collectibles/5_Gem_Collectible.5_Gem_Collectible_C|GetStone41 _returnvalue_8) (Math|Vector|MakeVector _returnvalue_5 _returnvalue_6 _returnvalue_4) "None" false)
            (Variables|Default|SetCurrent%20Value (+ (Variables|Default|GetCurrent%20Value) 5))
            (goto _label Reset)
            (else
              _)))
        (if (<= (Variables|Default|GetTemporary%20value) 75)
          (if (<= (Variables|Default|GetCurrent%20Value) (- (Variables|Default|GetTarget%20Value) 25))
            (bind _returnvalue_9 (Game|SpawnActorfromClass "/Game/Main/Blueprints/Collectibles/25-Gem-Collectible.25-Gem-Collectible_C" (Math|Transform|MakeTransform _returnvalue_3 "0, 0, 0" "1.000000,1.000000,1.000000") "Undefined" "MultiplyWithRoot" 0 0))
            (Physics|AddForce (Variables|/Game/Main/Blueprints/Collectibles/25-Gem-Collectible.25-Gem-Collectible_C|GetStone41 _returnvalue_9) (Math|Vector|MakeVector _returnvalue_5 _returnvalue_6 _returnvalue_4) "None" false)
            (Variables|Default|SetCurrent%20Value (+ (Variables|Default|GetCurrent%20Value) 25))
            (goto _label Reset)
            (else
              _)))
        (if (<= (Variables|Default|GetTemporary%20value) 100)
          (if (<= (Variables|Default|GetCurrent%20Value) (- (Variables|Default|GetTarget%20Value) 100))
            (bind _returnvalue_10 (Game|SpawnActorfromClass "/Game/Main/Blueprints/Collectibles/100-Gem-Collectible.100-Gem-Collectible_C" (Math|Transform|MakeTransform _returnvalue_3 "0, 0, 0" "1.000000,1.000000,1.000000") "Undefined" "MultiplyWithRoot" 0 0))
            (Physics|AddForce (Variables|/Game/Main/Blueprints/Collectibles/100-Gem-Collectible.100-Gem-Collectible_C|GetStone41 _returnvalue_10) (Math|Vector|MakeVector _returnvalue_5 _returnvalue_6 _returnvalue_4) "None" false)
            (Variables|Default|SetCurrent%20Value (+ (Variables|Default|GetCurrent%20Value) 100))
            (goto _label Reset)
            (else
              (goto _label_2)))
          (else
            (goto _label_2)))))))

(fn ConstructionScript)