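; Temporary spawner actor that bursts five random gem collectibles from its location, then destroys itself.
; On BeginPlay, each of five loop passes rolls evenly among the 1, 5, 25 and 100 gem collectible classes and spawns one.
; Each gem's stone component gets an added force with random horizontal spread and a set upward push, both scaled by a multiplier.
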(event EventBeginPlay
  (bind _returnvalue (Math|Random|RandomFloatinRange -8e+01 8e+01))
  (bind _returnvalue_2 (Math|Random|RandomFloatinRange -8e+01 8e+01))
  (bind _returnvalue_3 (Transformation|GetActorLocation))
  (bind _multiplier (Variables|Default|GetMultiplier))
  (bind _upwards_force (Variables|Default|GetUpwards%20Force))
  (bind _returnvalue_4 (* _upwards_force _multiplier))
  (bind _returnvalue_5 (* _returnvalue_2 _multiplier))
  (bind _returnvalue_6 (* _returnvalue _multiplier))
  (for _index (range 1 5)
    (Variables|Default|SetTemporary%20value (Math|Random|RandomIntegerinRange 1 4))
    (if (== (Variables|Default|GetTemporary%20value) 1)
      (bind _returnvalue_7 (Game|SpawnActorfromClass "/Game/Main/Blueprints/Collectibles/1_Gem_Collectible.1_Gem_Collectible_C" (Math|Transform|MakeTransform _returnvalue_3 "0, 0, 0" "1.000000,1.000000,1.000000") "Undefined" "MultiplyWithRoot" 0 0))
      (Physics|AddForce (Variables|/Game/Main/Blueprints/Collectibles/1_Gem_Collectible.1_Gem_Collectible_C|GetStone41 _returnvalue_7) (Math|Vector|MakeVector _returnvalue_5 _returnvalue_6 _returnvalue_4) "None" false)
      (elif (== (Variables|Default|GetTemporary%20value) 2)
        (bind _returnvalue_8 (Game|SpawnActorfromClass "/Game/Main/Blueprints/Collectibles/5_Gem_Collectible.5_Gem_Collectible_C" (Math|Transform|MakeTransform _returnvalue_3 "0, 0, 0" "1.000000,1.000000,1.000000") "Undefined" "MultiplyWithRoot" 0 0))
        (Physics|AddForce (Variables|/Game/Main/Blueprints/Collectibles/5_Gem_Collectible.5_Gem_Collectible_C|GetStone41 _returnvalue_8) (Math|Vector|MakeVector _returnvalue_5 _returnvalue_6 _returnvalue_4) "None" false)
        (elif (== (Variables|Default|GetTemporary%20value) 3)
          (bind _returnvalue_9 (Game|SpawnActorfromClass "/Game/Main/Blueprints/Collectibles/25-Gem-Collectible.25-Gem-Collectible_C" (Math|Transform|MakeTransform _returnvalue_3 "0, 0, 0" "1.000000,1.000000,1.000000") "Undefined" "MultiplyWithRoot" 0 0))
          (Physics|AddForce (Variables|/Game/Main/Blueprints/Collectibles/25-Gem-Collectible.25-Gem-Collectible_C|GetStone41 _returnvalue_9) (Math|Vector|MakeVector _returnvalue_5 _returnvalue_6 _returnvalue_4) "None" false)
          (elif (== (Variables|Default|GetTemporary%20value) 4)
            (bind _returnvalue_10 (Game|SpawnActorfromClass "/Game/Main/Blueprints/Collectibles/100-Gem-Collectible.100-Gem-Collectible_C" (Math|Transform|MakeTransform _returnvalue_3 "0, 0, 0" "1.000000,1.000000,1.000000") "Undefined" "MultiplyWithRoot" 0 0))
            (Physics|AddForce (Variables|/Game/Main/Blueprints/Collectibles/100-Gem-Collectible.100-Gem-Collectible_C|GetStone41 _returnvalue_10) (Math|Vector|MakeVector _returnvalue_5 _returnvalue_6 _returnvalue_4) "None" false))))))
  (Actor|DestroyActor))

(event Collision|EventActorBeginOverlap
  (params (OtherActor :type Actor%20Object%20Reference)))

(event EventTick
  (params (DeltaSeconds :type Float%20%28single-precision%29)))

(fn ConstructionScript)