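; Gem collectible pickup that adds its GemValue to the player's gem count.
; On begin play the stone gets a random rotation, then stops simulating physics after a five-second delay.
; Overlapping the collect trigger starts a move of the stone, passing the other actor's world location as a relative target.
; The gem count updates through Playing_Instance, a pickup sound plays and the actor destroys itself.
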(event OnComponentBeginOverlap(Sphere)
  (params (OverlappedComponent :type Primitive%20Component%20Object%20Reference) (OtherActor :type Actor%20Object%20Reference) (OtherComp :type Primitive%20Component%20Object%20Reference) (OtherBodyIndex :type Integer) (bFromSweep :type Boolean) (SweepResult :type Hit%20Result%20Structure%20%28by%20ref%29)))

(event OnComponentBeginOverlap(Trigger_collect_start)
  (params (OverlappedComponent :type Primitive%20Component%20Object%20Reference) (OtherActor :type Actor%20Object%20Reference) (OtherComp :type Primitive%20Component%20Object%20Reference) (OtherBodyIndex :type Integer) (bFromSweep :type Boolean) (SweepResult :type Hit%20Result%20Structure%20%28by%20ref%29))
  (Components|MoveComponentTo (Variables|Default|GetStone41) (Transformation|GetWorldLocation (Variables|/Script/Engine.Actor|GetRootComponent OtherActor)) "0, 0, 0" false false 0.2 false)
  (bind _asplaying_instance (Utilities|Casting|CastToPlaying_Instance (Game|GetGameInstance)))
  (Default|AddtoPlayerGemCount _asplaying_instance (Variables|Default|GetGem%20Value))
  (Audio|SpawnSound2D "/Game/Main/Sound_effects/Collectibles/Gem_pickup.Gem_pickup" 1.0 1.0 0.0 0)
  (Actor|DestroyActor))

(event EventBeginPlay
  (Transformation|AddWorldRotation (Variables|Default|GetStone41) (Math|Random|RandomRotator true) false false)
  (Utilities|FlowControl|Delay 5.0)
  (Physics|SetSimulatePhysics (Variables|Default|GetStone41) false))

(event Collision|EventActorBeginOverlap
  (params (OtherActor :type Actor%20Object%20Reference)))

(event EventTick
  (params (DeltaSeconds :type Float%20%28single-precision%29)))

(fn ConstructionScript)