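; Gem collectible that adds its value to the player's gem count when picked up.
; On spawn it gets a random rotation, registers its value in the level gem count on Playing_Instance, and stops simulating physics after a short timer.
; Any overlap on the collect trigger moves the stone toward the other actor's location, then re-enters the shared BeginPlay branch to credit the player, play a sound and destroy the gem.
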(event OnComponentBeginOverlap(Sphere)
  (params (OverlappedComponent :type Primitive%20Component%20Object%20Reference) (OtherActor :type Actor%20Object%20Reference) (OtherComp :type Primitive%20Component%20Object%20Reference) (OtherBodyIndex :type Integer) (bFromSweep :type Boolean) (SweepResult :type Hit%20Result%20Structure%20%28by%20ref%29)))

(event OnComponentBeginOverlap(Trigger_collect_start)
  (params (OverlappedComponent :type Primitive%20Component%20Object%20Reference) (OtherActor :type Actor%20Object%20Reference) (OtherComp :type Primitive%20Component%20Object%20Reference) (OtherBodyIndex :type Integer) (bFromSweep :type Boolean) (SweepResult :type Hit%20Result%20Structure%20%28by%20ref%29))
  (bind _gem_value (Variables|Default|GetGem%20Value))
  (Components|MoveComponentTo (Variables|Default|GetStone41) (Transformation|GetWorldLocation (Variables|/Script/Engine.Actor|GetRootComponent OtherActor)) "0, 0, 0" false false 0.2 false)
  (Variables|Default|SetCollected true)
  (bind _asplaying_instance (Utilities|Casting|CastToPlaying_Instance (Game|GetGameInstance)))
  (if (Variables|Default|GetCollected)
    (Default|AddtoPlayerGemCount _asplaying_instance _gem_value)
    (Audio|SpawnSound2D "/Game/Main/Sound_effects/Collectibles/Gem_pickup.Gem_pickup" 1.0 1.0 0.0 0)
    (Actor|DestroyActor)
    (else
      (Default|LevelGemCount _asplaying_instance _gem_value))))

(event Custom|Stop%20Physics
  ;[0.15 0.15 0.15 0.5] Stop physics after 5 seconds
  (Physics|SetSimulatePhysics (Variables|Default|GetStone41) false))

(event EventBeginPlay
  (bind _gem_value (Variables|Default|GetGem%20Value))
  ;[0.15 0.15 0.15 0.5] Give random rotation upon being spawned
  (Transformation|AddWorldRotation (Variables|Default|GetStone41) (Math|Random|RandomRotator true) false false)
  (Utilities|Time|SetTimerbyFunctionName 0 "Stop Physics" 5.0)
  (bind _asplaying_instance (Utilities|Casting|CastToPlaying_Instance (Game|GetGameInstance)))
  (if (Variables|Default|GetCollected)
    (Default|AddtoPlayerGemCount _asplaying_instance _gem_value)
    (Audio|SpawnSound2D "/Game/Main/Sound_effects/Collectibles/Gem_pickup.Gem_pickup" 1.0 1.0 0.0 0)
    (Actor|DestroyActor)
    (else
      (Default|LevelGemCount _asplaying_instance _gem_value))))

(fn ConstructionScript)