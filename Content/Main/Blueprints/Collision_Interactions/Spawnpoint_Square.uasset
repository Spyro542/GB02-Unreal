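; Spawnpoint actor that registers itself with the player and provides a respawn function.
; Both begin and end overlap with a PlayerV3 pass this actor to that player's Spawnpoint function.
; PlayerRespawn destroys the given player actor and spawns a fresh PlayerV3 at this actor's Capsule location and rotation, adjusting for collisions but always spawning.
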(event Collision|EventActorBeginOverlap
  (params (OtherActor :type Actor%20Object%20Reference))
  (bind _asplayer_v3 (Utilities|Casting|CastToPlayerV3 OtherActor))
  (Default|Spawnpoint _asplayer_v3 self))

(event Collision|EventActorEndOverlap
  (params (OtherActor :type Actor%20Object%20Reference))
  (bind _asplayer_v3 (Utilities|Casting|CastToPlayerV3 OtherActor))
  (Default|Spawnpoint _asplayer_v3 self))

(fn ConstructionScript)

(fn PlayerRespawn
  (params (Player%20Actor :type Actor%20Object%20Reference))
  (bind _capsule (Variables|Default|GetCapsule))
  (Actor|DestroyActor Player%20Actor)
  (Game|SpawnActorfromClass "/Game/Main/Blueprints/Player/PlayerV3.PlayerV3_C" (Math|Transform|MakeTransform (Transformation|GetWorldLocation _capsule) (Transformation|GetWorldRotation _capsule) "1.000000,1.000000,1.000000") "AdjustIfPossibleButAlwaysSpawn" "MultiplyWithRoot" 0 0))