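; BP_World_Gate is a level exit gate that opens the next level once the player has enough gems.
; Each Tick it compares player and Level 1 gem counts from Playing_Instance, hiding the condition display and showing the transfer trigger when met.
; Overlapping the trigger repeats the check, then loads NextLevel by object reference.
; The overlap does not filter the overlapping actor, and the threshold always uses Level1GemCount.
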(event OnComponentBeginOverlap(LevelTransferTrigger)
  (params (OverlappedComponent :type Primitive%20Component%20Object%20Reference) (OtherActor :type Actor%20Object%20Reference) (OtherComp :type Primitive%20Component%20Object%20Reference) (OtherBodyIndex :type Integer) (bFromSweep :type Boolean) (SweepResult :type Hit%20Result%20Structure%20%28by%20ref%29))
  (bind _asplaying_instance (Utilities|Casting|CastToPlaying_Instance (Game|GetGameInstance)))
  (if (<= (Variables|/Game/Main/Game_Handling/Playing_Instance.Playing_Instance_C|GetLevel%201%20Gem%20Count _asplaying_instance) (Variables|/Game/Main/Game_Handling/Playing_Instance.Playing_Instance_C|GetPlayer%20Gem%20Count _asplaying_instance))
    (Game|OpenLevel(byObjectReference) (Variables|Stats|GetNext%20Level))))

(event EventBeginPlay)

(event Collision|EventActorBeginOverlap
  (params (OtherActor :type Actor%20Object%20Reference)))

(event EventTick
  (params (DeltaSeconds :type Float%20%28single-precision%29))
  (bind _asplaying_instance (Utilities|Casting|CastToPlaying_Instance (Game|GetGameInstance)))
  (if (<= (Variables|/Game/Main/Game_Handling/Playing_Instance.Playing_Instance_C|GetLevel%201%20Gem%20Count _asplaying_instance) (Variables|/Game/Main/Game_Handling/Playing_Instance.Playing_Instance_C|GetPlayer%20Gem%20Count _asplaying_instance))
    (Development|SetHiddeninGame (Variables|Default|GetTrigger%20Condition%20Display) true false)
    (Rendering|SetVisibility (Variables|Default|GetLevel%20Transfer%20Trigger) true false)))

(fn ConstructionScript)