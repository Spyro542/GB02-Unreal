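; Spawnpoint actor that marks respawn locations for PlayerV3 characters.
; Both beginning and ending an overlap with a PlayerV3 pass this actor to that player's Spawnpoint call.
; PlayerRespawn destroys the given player actor and spawns a fresh PlayerV3 at the spawnpoint's location and rotation, adjusting for collisions but always spawning.
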(event Collision|EventActorEndOverlap
  (params (OtherActor :type Actor%20Object%20Reference))
  (bind _asplayer_v3 (Utilities|Casting|CastToPlayerV3 OtherActor))
  (Default|Spawnpoint _asplayer_v3 self))

(event Collision|EventActorBeginOverlap
  (params (OtherActor :type Actor%20Object%20Reference))
  (bind _asplayer_v3 (Utilities|Casting|CastToPlayerV3 OtherActor))
  (Default|Spawnpoint _asplayer_v3 self))

(event EventTick
  (params (DeltaSeconds :type Float%20%28single-precision%29)))

(fn ConstructionScript)

(fn PlayerRespawn
  (params (Player%20Actor :type Actor%20Object%20Reference))
  (Actor|DestroyActor Player%20Actor)
  (Game|SpawnActorfromClass "/Game/Main/Blueprints/Player/PlayerV3.PlayerV3_C" (Math|Transform|MakeTransform (Transformation|GetActorLocation) (Transformation|GetActorRotation) "1.000000,1.000000,1.000000") "AdjustIfPossibleButAlwaysSpawn" "MultiplyWithRoot" 0 0))